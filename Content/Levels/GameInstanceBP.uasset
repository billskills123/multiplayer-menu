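; Game Instance Blueprint that handles network and travel failures in a multiplayer session game.
; Both error events create an ErrorUI widget and set its text to the failure type.
; After a short delay, each destroys the session and opens MainMenu whether that succeeds or fails, so players outside a session also return to the menu.
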(event `self.HandleNetworkError`
  (params (FailureType :type "ENetworkFailure Enum" :default "NetDriverAlreadyExists") (bIsServer :type Boolean))
  ;[1 1 1] Handle network errors. If the player has managed to make it into the session destroy the session and return them back to the main menu.
  ; If they are not in the session leaving the session will fail but still return the player back to the main menu
  (bind _returnvalue (`|CreateWidget` "/Game/UI/ErrorUI.ErrorUI_C" (`GameplayStatics.GetPlayerController` 0)))
  (`/Game/UI/ErrorUI.Change Error Text` _returnvalue (`KismetTextLibrary.Conv_StringToText` (`KismetStringLibrary.Concat_StrStr` "Error: " (`|GetEnumeratorNameAsString` FailureType))))
  (`KismetSystemLibrary.Delay` 2.5)
  (`DestroySessionCallbackProxy.DestroySession` (`GameplayStatics.GetPlayerController` 0)
    (:`OnSuccess`
      _)
    (:`OnFailure`
      _))
  (`GameplayStatics.OpenLevel` "MainMenu"))

(event `self.HandleTravelError`
  (params (FailureType :type "ETravelFailure Enum" :default "NoLevel"))
  ;[1 1 1] Handle network errors. If the player has managed to make it into the session destroy the session and return them back to the main menu.
  ; If they are not in the session leaving the session will fail but still return the player back to the main menu
  (bind _returnvalue (`|CreateWidget` "/Game/UI/ErrorUI.ErrorUI_C" (`GameplayStatics.GetPlayerController` 0)))
  (`/Game/UI/ErrorUI.Change Error Text` _returnvalue (`KismetTextLibrary.Conv_StringToText` (`KismetStringLibrary.Concat_StrStr` "Error: " (`|GetEnumeratorNameAsString` FailureType))))
  (`KismetSystemLibrary.Delay` 2.5)
  (`DestroySessionCallbackProxy.DestroySession` (`GameplayStatics.GetPlayerController` 0)
    (:`OnSuccess`
      _)
    (:`OnFailure`
      _))
  (`GameplayStatics.OpenLevel` "MainMenu"))